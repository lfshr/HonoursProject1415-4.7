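; Player character Blueprint that handles movement, camera look and sprinting, and issues commands to OwenController actors.
; Axis inputs drive movement and look, with sprint changing CurrentSpeed, which scales the movement input rather than setting a movement component speed.
; G and V find every OwenController and tell it to move behind the player or to a tree.
; On BeginPlay, GetTreeSpawners gathers overlapping tree spawners, whose names are printed for debugging.
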(event EventBeginPlay
  (bind _tree_spawners (CallFunction|GetTreeSpawners))
  (for _array_element _tree_spawners
    (Development|PrintString (Utilities|GetDisplayName _array_element))))

(event Input|ActionEvents|InputActionSprint
  ;[1 1 1] Sprint Logic
  (:Pressed
    (Variables|Default|SetcurrentSpeed (Variables|Default|GetsprintSpeed)))
  (:Released
    (Variables|Default|SetcurrentSpeed 0.5)))

(event Input|AxisEvents|InputAxisMoveHorizontal
  (params (AxisValue :type Float%20%28single-precision%29))
  ;[1 1 1] Movement Logic
  (Pawn|Input|AddMovementInput (Transformation|GetActorRightVector) (* (Variables|Default|GetcurrentSpeed) AxisValue) false))

(event Input|AxisEvents|InputAxisLookHorizontal
  (params (AxisValue :type Float%20%28single-precision%29))
  ;[1 1 1] Look Logic
  (Pawn|Input|AddControllerYawInput (* AxisValue (Variables|Default|GetturnSpeed))))

(event Input|AxisEvents|InputAxisMoveForward
  (params (AxisValue :type Float%20%28single-precision%29))
  ;[1 1 1] Movement Logic
  (Pawn|Input|AddMovementInput (Transformation|GetActorForwardVector) (* AxisValue (Variables|Default|GetcurrentSpeed)) false))

(event Input|AxisEvents|InputAxisLookVertical
  (params (AxisValue :type Float%20%28single-precision%29))
  ;[1 1 1] Look Logic
  (Pawn|Input|AddControllerPitchInput (* (Variables|Default|GetturnSpeed) AxisValue)))

(event Input|KeyboardEvents|G
  (:Pressed
    (bind _outactors (Actor|GetAllActorsOfClass "/Game/HonoursContent/AI/owenController.owenController_C"))
    (for _array_element _outactors
      (bind _asowen_controller (Utilities|Casting|CastToowenController _array_element))
      (Default|MoveBehindPlayer _asowen_controller))))

(event Input|KeyboardEvents|V
  (:Pressed
    (bind _outactors (Actor|GetAllActorsOfClass "/Game/HonoursContent/AI/owenController.owenController_C"))
    (for _array_element _outactors
      (bind _asowen_controller (Utilities|Casting|CastToowenController _array_element))
      (Default|MovetoTree _asowen_controller))))

(fn ConstructionScript)

(fn GetTreeSpawners
  (bind _self self)
  (bind _overlappingactors (Collision|GetOverlappingActors _self "/Game/HonoursContent/Blueprints/tree_spawner.tree_spawner_C" :!class /Script/Engine.PrimitiveComponent))
  (for _array_element _overlappingactors
    (Development|PrintString (Utilities|GetDisplayName _array_element)))
  (return _overlappingactors))
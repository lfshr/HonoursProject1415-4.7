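; Tree spawner that supplies a spawn point on its far side from the player.
; GetSpawnLocation finds the first PlayerCharacter, extends the line from the player through this actor by SpawnDistance, and projects that point onto the navmesh.
; It only computes the location and spawns nothing itself; the construction script is empty and the event graph holds only unreachable nodes.
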(fn ConstructionScript)

(fn GetSpawnLocation
  (bind _returnvalue (Transformation|GetActorLocation))
  (bind _outactors (Actor|GetAllActorsOfClass "/Game/HonoursContent/Blueprints/playerCharacter.playerCharacter_C"))
  (bind _asplayer_character (Utilities|Casting|CastToplayerCharacter (Utilities|Array|Get(acopy) _outactors))
    (:then
      (return (AI|Navigation|ProjectPointtoNavigation (+ (Transformation|GetActorLocation _asplayer_character) (* (Math|Vector|GetForwardVector (Math|Rotator|FindLookatRotation (Transformation|GetActorLocation _asplayer_character) _returnvalue)) (+ (Math|Vector|VectorLength (- (Transformation|GetActorLocation _asplayer_character) _returnvalue)) (Variables|Default|GetspawnDistance)))) 0 0)))
    (:CastFailed
      (Development|PrintString "Failed to cast to playerCharacter on Get Spawn Location"))))
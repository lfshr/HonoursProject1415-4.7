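; Interactive wooden door that swings open or closed when the player presses the action button.
; Front and back trigger overlaps enable input and pick the swing direction, which the door type can lock to clockwise or anti-clockwise.
; Two timelines lerp relative rotation toward yaws derived from the open rotation, reversing to close.
; Input is never disabled, so an open door closes on a press even outside the triggers.
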(event OnComponentBeginOverlap(trigger_front)
  (params (OtherActor :type Actor%20Object%20Reference) (OtherComp :type Primitive%20Component%20Object%20Reference) (OtherBodyIndex :type Integer) (bFromSweep :type Boolean) (SweepResult :type Hit%20Result%20Structure%20%28by%20ref%29))
  ;[1 1 1] Front Collider Collison
  (Variables|Default|Settrigger_front_overlap true)
  (Input|EnableInput (Game|GetPlayerController 0)))

(event OnComponentEndOverlap(trigger_back)
  (params (OtherActor :type Actor%20Object%20Reference) (OtherComp :type Primitive%20Component%20Object%20Reference) (OtherBodyIndex :type Integer))
  ;[1 1 1] Back Collider Collision
  (Variables|Default|Settrigger_back_overlap false))

(event OnComponentBeginOverlap(trigger_back)
  (params (OtherActor :type Actor%20Object%20Reference) (OtherComp :type Primitive%20Component%20Object%20Reference) (OtherBodyIndex :type Integer) (bFromSweep :type Boolean) (SweepResult :type Hit%20Result%20Structure%20%28by%20ref%29))
  ;[1 1 1] Back Collider Collision
  (Variables|Default|Settrigger_back_overlap true)
  (Input|EnableInput (Game|GetPlayerController 0)))

(event OnComponentEndOverlap(trigger_front)
  (params (OtherActor :type Actor%20Object%20Reference) (OtherComp :type Primitive%20Component%20Object%20Reference) (OtherBodyIndex :type Integer))
  ;[1 1 1] Front Collider Collison
  (Variables|Default|Settrigger_front_overlap false))

(event EventBeginPlay
  (bind _openrotation (Variables|Default|GetopenRotation))
  ;[1 1 1] On Begin Play
  (Variables|Default|SetopenForward (Class|KismetMathLibrary|MakeRot 0.0 (- 3.6e+02 _openrotation) 0.0))
  (Variables|Default|SetopenBackward (Class|KismetMathLibrary|MakeRot 0.0 _openrotation 0.0)))

(event Input|ActionEvents|InputActionactionButton
  ;[1 1 1] Button Press Logic
  (:Pressed
    (if (Variables|Default|GetisOpenForward)
      (Utilities|FlowControl|Sequence
        (:then_0
          ;[1 1 1] Reset Open Status
          (Variables|Default|SetisOpenForward false :!label _label)
          (Variables|Default|SetisOpenBackward false))
        (:then_1
          ;[1 1 1] Open Forward
          (bind (_direction _driver) (Timeline|Timeline%20Open Reverse)
            (:Update
              (Transformation|SetRelativeRotation (Math|Rotator|Lerp(Rotator) (Variables|Default|GetdefaultRotation) (Variables|Default|GetopenForward) _driver true) false))
            (:Finished
              (switch Utilities|FlowControl|Switch|SwitchonETimelineDirection _direction
                (:Forward
                  (Variables|Default|SetisOpenForward true))
                (:Backward
                  (goto _label)))))))
      (elif (Variables|Default|GetisOpenBackward)
        (Utilities|FlowControl|Sequence
          (:then_0
            (goto _label))
          (:then_1
            ;[1 1 1] Open Backwards
            (bind (_direction_2 _driver_2) (Timeline|Timeline%20Open%20Backwards Reverse)
              (:Update
                (Transformation|SetRelativeRotation (Math|Rotator|Lerp(Rotator) (Variables|Default|GetdefaultRotation) (Variables|Default|GetopenBackward) _driver_2 true) false))
              (:Finished
                (switch Utilities|FlowControl|Switch|SwitchonETimelineDirection _direction_2
                  (:Forward
                    (Variables|Default|SetisOpenBackward true))
                  (:Backward
                    (goto _label)))))))
        (elif (Variables|Default|Gettrigger_front_overlap)
          ;[1 1 1] Attempt to open Forward
          (switch Utilities|FlowControl|Switch|SwitchonDoorType (Variables|Default|GetDoorType)
            (:NewEnumerator0
              (Timeline|Timeline%20Open Play))
            (:NewEnumerator1
              (Timeline|Timeline%20Open%20Backwards Play))
            (:NewEnumerator2
              (Timeline|Timeline%20Open Play)))
          (elif (Variables|Default|Gettrigger_back_overlap)
            ;[1 1 1] Attempt to open Backward
            (switch Utilities|FlowControl|Switch|SwitchonDoorType (Variables|Default|GetDoorType)
              (:NewEnumerator0
                (Timeline|Timeline%20Open%20Backwards Play))
              (:NewEnumerator1
                (Timeline|Timeline%20Open%20Backwards Play))
              (:NewEnumerator2
                (Timeline|Timeline%20Open Play)))))))))

(fn ConstructionScript)
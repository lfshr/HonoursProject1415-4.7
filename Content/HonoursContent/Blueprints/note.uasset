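; Collectible note actor that the player picks up with the action button while standing near it.
; Overlap events on PlayerRangeChecker track whether the player character is in range and enable input on the note for that player's controller.
; Pressing the action button in range fires the NoteFound dispatcher and destroys the actor; input is never explicitly disabled when the player leaves.
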(event OnComponentBeginOverlap(playerRangeChecker)
  (params (OtherActor :type Actor%20Object%20Reference) (OtherComp :type Primitive%20Component%20Object%20Reference) (OtherBodyIndex :type Integer) (bFromSweep :type Boolean) (SweepResult :type Hit%20Result%20Structure%20%28by%20ref%29))
  ;[1 1 1] Player Overlapping Calculations
  (if (== (Utilities|GetClass OtherActor) "/Game/HonoursContent/Blueprints/playerCharacter.playerCharacter_C")
    (Variables|Default|SetplayerInRange true)
    (bind _asplayer_character (Utilities|Casting|CastToplayerCharacter OtherActor))
    (bind _returnvalue (Utilities|Casting|CastToPlayerController (Pawn|GetController _asplayer_character)))
    (Input|EnableInput _returnvalue)))

(event OnComponentEndOverlap(playerRangeChecker)
  (params (OtherActor :type Actor%20Object%20Reference) (OtherComp :type Primitive%20Component%20Object%20Reference) (OtherBodyIndex :type Integer))
  ;[1 1 1] Player Overlapping Calculations
  (if (== (Utilities|GetClass OtherActor) "/Game/HonoursContent/Blueprints/playerCharacter.playerCharacter_C")
    (Variables|Default|SetplayerInRange false)))

(event EventBeginPlay)

(event EventActorBeginOverlap
  (params (OtherActor :type Actor%20Object%20Reference)))

(event EventTick
  (params (DeltaSeconds :type Float%20%28single-precision%29)))

(event Input|ActionEvents|InputActionactionButton
  (:Pressed
    (if (Variables|Default|GetplayerInRange)
      (Default|CallNoteFound)
      (Actor|DestroyActor))))

(fn ConstructionScript)